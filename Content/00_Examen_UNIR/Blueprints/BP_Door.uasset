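; BP_Door is a sliding double door that opens when its linked button is active and the player has collected enough keys.
; On BeginPlay it caches the panel positions and player character, then binds to the button's active-state change.
; Each change checks KeysCollected against RequiredKeys, printing a Spanish on-screen hint if short.
; Otherwise a Timeline lerps both panels apart, or reverses to close them when the button is inactive.
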(event `self.ReceiveBeginPlay`
  (set `self.initPosRDoor` (`SceneComponent.RelativeLocation` (`self.RightDoor`)))
  (set `self.initPosLDoor` (`SceneComponent.RelativeLocation` (`self.LeftDoor`)))
  (bind _asbp_third_person_character (cast `/Game/ThirdPerson/Blueprints/BP_ThirdPersonCharacter` (`GameplayStatics.GetPlayerCharacter` 0)))
  (set `self.PlayerCharacterRef` _asbp_third_person_character)
  (bind _button (`self.Button`)
    (:`then`
      (add `/Game/00_Examen_UNIR/Blueprints/BP_FloorButton.ChangeActiveState` _button (delegate `VerifyState`)))
    (:`else`)))

(event `VerifyState`
  (`self.VerifyConditions`))

(event `OpenDoor`
  (bind _initposldoor (`self.initPosLDoor`))
  (bind _initposrdoor (`self.initPosRDoor`))
  (bind (_direction _newtrack_0) (`Timeline|Timeline` :!label _label)
    (:`Update`
      (`SceneComponent.K2_SetRelativeLocation` (`self.RightDoor`) (`KismetMathLibrary.VLerp` _initposrdoor (+ _initposrdoor (90.0 0.0 0.0)) _newtrack_0) false false)
      (`SceneComponent.K2_SetRelativeLocation` (`self.LeftDoor`) (`KismetMathLibrary.VLerp` _initposldoor (+ _initposldoor (-90.0 0.0 0.0)) _newtrack_0) false false))))

(event `CloseDoor`
  (goto _label :!via `Reverse`))

(event `VerifyConditions`
  (if (>= (`/Game/ThirdPerson/Blueprints/BP_ThirdPersonCharacter.KeysCollected` (`self.PlayerCharacterRef`)) (`self.RequiredKeys`))
    (if (`/Game/00_Examen_UNIR/Blueprints/BP_FloorButton.isActive` (`self.Button`))
      (`self.OpenDoor`)
      (else
        (`self.CloseDoor`)))
    (else
      (`KismetSystemLibrary.PrintString` (`KismetStringLibrary.Concat_StrStr` "Necesitas " (`KismetStringLibrary.Conv_IntToString` (`self.RequiredKeys`)) " llave(s) para abrir!")))))

(fn `UserConstructionScript`)