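; BP_FloorButton is an interactive floor button that toggles an active state when the player presses E nearby.
; Box overlaps with BP_ThirdPersonCharacter enable and disable the actor's input for player controller 0, so the key works only inside the trigger.
; Each press flips IsActive, swaps the Hieroglyph between emission on and off materials, and calls the ChangeActiveState dispatcher to broadcast the change.
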(event `self.ReceiveBeginPlay`
  (`PrimitiveComponent.SetMaterial` (`self.Hieroglyph`) 0 "/Game/00_Examen_UNIR/Materials/M_Emission_Off.M_Emission_Off"))

(event `self.Box.OnComponentBeginOverlap`
  (params (OverlappedComponent :type "PrimitiveComponent Object Reference") (OtherActor :type "Actor Object Reference") (OtherComp :type "PrimitiveComponent Object Reference") (OtherBodyIndex :type Integer) (bFromSweep :type Boolean) (SweepResult :type "HitResult Structure (by ref)"))
  (cast `/Game/ThirdPerson/Blueprints/BP_ThirdPersonCharacter` OtherActor)
  (`self.EnableInput` (`GameplayStatics.GetPlayerController` 0)))

(event `self.Box.OnComponentEndOverlap`
  (params (OverlappedComponent :type "PrimitiveComponent Object Reference") (OtherActor :type "Actor Object Reference") (OtherComp :type "PrimitiveComponent Object Reference") (OtherBodyIndex :type Integer))
  (cast `/Game/ThirdPerson/Blueprints/BP_ThirdPersonCharacter` OtherActor)
  (`self.DisableInput` (`GameplayStatics.GetPlayerController` 0)))

(event `Key|E`
  (params (Key :type "Key Structure"))
  (:`Pressed`
    (bind _output_get (set `self.isActive` (not (`self.isActive`))))
    (if _output_get
      (`PrimitiveComponent.SetMaterial` (`self.Hieroglyph`) 0 "/Game/00_Examen_UNIR/Materials/M_Emission_On.M_Emission_On")
      (else
        (`PrimitiveComponent.SetMaterial` (`self.Hieroglyph`) 0 "/Game/00_Examen_UNIR/Materials/M_Emission_Off.M_Emission_Off")))
    (`self.ChangeActiveState`)))

(fn `UserConstructionScript`)